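; BP_Platform is a trap platform actor that reacts when BP_MyPlayer overlaps its Box, with behavior chosen by PlatformType.
; Falling Platform drops the Cube via physics simulation after a short delay, then teleports it back to the transform cached at BeginPlay.
; Squid Game Bridge drops only when flagged FakePlatform, then destroys the actor.
; The construction script sets the Cube's material from a random or chosen color.
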(event OnComponentBeginOverlap(Box)
  (params (OverlappedComponent :type Primitive%20Component%20Object%20Reference) (OtherActor :type Actor%20Object%20Reference) (OtherComp :type Primitive%20Component%20Object%20Reference) (OtherBodyIndex :type Integer) (bFromSweep :type Boolean) (SweepResult :type Hit%20Result%20Structure%20%28by%20ref%29))
  (Utilities|Casting|CastToBP_MyPlayer OtherActor)
  (switch Utilities|FlowControl|Switch|SwitchonE_PlatformType (Variables|Default|GetPlatformType)
    (:NewEnumerator0
      (Utilities|FlowControl|Delay 1.0)
      (Physics|SetSimulatePhysics (Variables|Default|GetCube) true)
      (Utilities|FlowControl|Delay 5.0)
      (Physics|SetSimulatePhysics (Variables|Default|GetCube) false)
      (Transformation|SetWorldTransform (Variables|Default|GetCube) (Variables|Default|GetdefaultTransform) false true))
    (:NewEnumerator1
      (if (Variables|Default|GetfakePlatform?)
        (Physics|SetSimulatePhysics (Variables|Default|GetCube) true)
        (Utilities|FlowControl|Delay 5.0)
        (Actor|DestroyActor)))))

(event EventBeginPlay
  (Variables|Default|SetdefaultTransform (Transformation|GetWorldTransform (Variables|Default|GetCube))))

(fn ConstructionScript
  (if (Variables|Default|GetRandomize%20Colors?)
    (switch int (Math|Random|RandomIntegerinRange 0 4)
      (:0
        (Variables|Default|SetMaterialToSet "/Game/Blueprints/Materials/M_Orange.M_Orange" :!label _label))
      (:1
        (Variables|Default|SetMaterialToSet "/Game/Blueprints/Materials/M_Blue.M_Blue" :!label _label_2))
      (:2
        (Variables|Default|SetMaterialToSet "/Game/Blueprints/Materials/M_Violet.M_Violet" :!label _label_3))
      (:3
        (Variables|Default|SetMaterialToSet "/Game/Blueprints/Materials/M_Green.M_Green" :!label _label_4))
      (:4
        (Variables|Default|SetMaterialToSet "/Game/Blueprints/Materials/M_Yellow.M_Yellow" :!label _label_5)))
    (else
      (switch Utilities|FlowControl|Switch|SwitchonE_Color (Variables|Default|GetColor)
        (:NewEnumerator0
          (goto _label))
        (:NewEnumerator1
          (goto _label_2))
        (:NewEnumerator2
          (goto _label_3))
        (:NewEnumerator3
          (goto _label_4))
        (:NewEnumerator4
          (goto _label_5)))))
  (Rendering|Material|SetMaterial (Variables|Default|GetCube) 0 (Variables|Default|GetMaterialToSet)))