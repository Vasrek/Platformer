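; BP_Door is a door actor that swings open by rotating 125 degrees in yaw from its placed rotation.
; BeginPlay caches the default rotation and computes the target rotation.
; OpenDoor starts a fast looping timer that calls Open, which eases the actor toward the target with RInterpTo at a Speed variable.
; The timer clears itself once the rotation is within tolerance, so no Tick is used.
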(event Custom|OpenDoor
  (Utilities|Time|SetTimerbyFunctionName 0 "Open" 0.01 true))

(event EventBeginPlay
  (|CallParentFunction)
  (bind _output_get (Variables|Default|SetDefaultRotation (Transformation|GetActorRotation)))
  (Variables|Default|SetFinalRotation (Math|Rotator|MakeRotator (.Roll (Math|Rotator|BreakRotator _output_get)) (.Pitch (Math|Rotator|BreakRotator _output_get)) (+ (.Yaw (Math|Rotator|BreakRotator _output_get)) 125.0))))

(event Collision|EventActorBeginOverlap
  (params (OtherActor :type Actor%20Object%20Reference))
  (|CallParentFunction OtherActor) ; This node is disabled and will not be called.\nDrag off pins to build functionality.
)

(event EventTick
  (params (DeltaSeconds :type Float%20%28single-precision%29))
  (|CallParentFunction DeltaSeconds) ; This node is disabled and will not be called.\nDrag off pins to build functionality.
)

(fn ConstructionScript
  (|CallParentFunction))

(fn Open
  (bind _returnvalue (Transformation|GetActorRotation))
  (bind _returnvalue_2 (Utilities|Time|GetWorldDeltaSeconds))
  (bind _finalrotation (Variables|Default|GetFinalRotation))
  (bind _speed (Variables|Default|GetSpeed))
  (bind _returnvalue_3 (Math|Interpolation|RInterpTo _returnvalue _finalrotation _returnvalue_2 _speed))
  (Transformation|SetActorRotation _returnvalue_3)
  (if (Utilities|Operators|EqualEqual _returnvalue_3 (Variables|Default|GetFinalRotation) 2.0)
    (Utilities|Time|ClearTimerbyFunctionName 0 "Open")))