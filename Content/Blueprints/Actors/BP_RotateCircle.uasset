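; BP_RotateCircle is an actor with a colored Cylinder that spins continuously around the vertical axis.
; The construction script applies one of five color materials to the Cylinder, either picked at random when RandomizeColors is set or chosen by the Color variable.
; BeginPlay gives the Cylinder a random starting yaw, and Tick adds a fixed yaw step each frame, so spin speed depends on frame rate.
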(event EventTick
  (params (DeltaSeconds :type Float%20%28single-precision%29))
  (bind _cylinder (Variables|Default|GetCylinder))
  (Transformation|SetWorldRotation _cylinder (Math|Rotator|MakeRotator 0.0 0.0 (+ (.yaw (Transformation|GetWorldRotation _cylinder)) 1.0)) false false))

(event EventBeginPlay
  (Transformation|SetWorldRotation (Variables|Default|GetCylinder) (Math|Rotator|MakeRotator 0.0 0.0 (Math|Random|RandomFloatinRange 0.0 3.6e+02)) false false))

(fn ConstructionScript
  (if (Variables|Default|GetRandomizeColors?)
    (switch int (Math|Random|RandomIntegerinRange 0 4)
      (:0
        (Variables|Default|SetMaterialToSet "/Game/Blueprints/Materials/M_Orange.M_Orange" :!label _label))
      (:1
        (Variables|Default|SetMaterialToSet "/Game/Blueprints/Materials/M_Blue.M_Blue" :!label _label_2))
      (:2
        (Variables|Default|SetMaterialToSet "/Game/Blueprints/Materials/M_Violet.M_Violet" :!label _label_3))
      (:3
        (Variables|Default|SetMaterialToSet "/Game/Blueprints/Materials/M_Green.M_Green" :!label _label_4))
      (:4
        (Variables|Default|SetMaterialToSet "/Game/Blueprints/Materials/M_Yellow.M_Yellow" :!label _label_5)))
    (else
      (switch Utilities|FlowControl|Switch|SwitchonE_Color (Variables|Default|GetColor)
        (:NewEnumerator0
          (goto _label))
        (:NewEnumerator1
          (goto _label_2))
        (:NewEnumerator2
          (goto _label_3))
        (:NewEnumerator3
          (goto _label_4))
        (:NewEnumerator4
          (goto _label_5)))))
  (Rendering|Material|SetMaterial (Variables|Default|GetCylinder) 0 (Variables|Default|GetMaterialToSet)))